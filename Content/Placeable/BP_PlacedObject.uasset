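; Placeable product actor that can be repositioned on the floor plane it was placed on from a screen position.
; Its construction script applies the mesh from a product asset reference and sizes a base plate from that asset's plate scale.
; SetPlaceablePosition deprojects the screen point, line-traces for objects, and moves the Placeable component to the hit only when it strikes BPPlane.
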(event EventBeginPlay)

(event Collision|EventActorBeginOverlap
  (params (OtherActor :type Actor%20Object%20Reference)))

(event EventTick
  (params (DeltaSeconds :type Float%20%28single-precision%29)))

(fn ConstructionScript
  (CallFunction|AssignProductAsset))

(fn AssignProductAsset
  (bind _bp_productassetref (Variables|Default|GetBP_ProductAssetRef))
  (bind _platescale (Variables|/Game/Placeable/BP_ProductAssetRef.BP_ProductAssetRef_C|GetPlateScale _bp_productassetref))
  (Components|StaticMesh|SetStaticMesh (Variables|Default|GetSM_Object) (Variables|/Game/Placeable/BP_ProductAssetRef.BP_ProductAssetRef_C|GetStataicMesh _bp_productassetref))
  (Transformation|SetWorldScale3D (Variables|Default|GetSM_Plate) (Math|Vector|MakeVector _platescale _platescale 0.0)))

(fn SetPlaceablePosition
  (params (vector2 :type Vector%202D%20Structure))
  (bind _returnvalue (Game|GetPlayerController 0))
  (bind (_worldposition _worlddirection) (Class|GameplayStatics|DeprojectScreentoWorld _returnvalue vector2))
  (bind (_outhit _returnvalue_2) (Collision|LineTraceForObjects _worldposition (+ _worldposition (* _worlddirection 1e+03)) (Utilities|Array|MakeArray "ObjectTypeQuery1" "ObjectTypeQuery2" "ObjectTypeQuery3" "ObjectTypeQuery4" "ObjectTypeQuery5" "ObjectTypeQuery6") false 0 "None"))
  (if _returnvalue_2
    ;[0.15 0.15 0.15 0.5] 지금 히트 하고 있는 대상이 오브젝트를 배치했던 해당 바닥이 맞는지 확인
    (if (== (.HitActor (Collision|BreakHitResult _outhit)) (Variables|Default|GetBP_Plane))
      (Transformation|SetWorldLocation (Variables|Default|GetPlaceable) (.Location (Collision|BreakHitResult _outhit)) false false))))